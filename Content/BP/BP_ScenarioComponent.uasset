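; BP_ScenarioComponent runs numbered scenario commands that drive the main UI and scene progression.
; Init caches MainUI from BP_MainGameMode, and ActivateAddon switches on an integer code to show or hide the player and mate pictures, toggle editing and clickability, or reset the player's picture.
; SceneCounter selects each scene's mate texture and editable element set.
; Other codes advance that counter or open the ending level.
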(event `Init`
  (bind _asbp_main_game_mode (cast `/Game/BP/BP_MainGameMode` (`GameplayStatics.GetGameMode`)))
  (bind _output_get (set `self.As BP Main Game Mode` _asbp_main_game_mode))
  (set `self.Main UI` (`/Game/BP/BP_MainGameMode.MainUI` _output_get)))

(event `ActivateAddon`
  (params (NewParam :type Integer))
  (bind _main_ui (`self.Main UI`))
  (bind _output_elementset (break `/Game/Data/AvailableElentSet` (`|GetArrayItem` (`self.AvaliableElementSets`) (`self.SceneCounter`))))
  (switch `int` NewParam
    (:`1`
      ;[1 1 1] 1 Show My Picture
      (`/Game/UI/WBP_MainScreen.ShowMyPicture` (`self.Main UI`) true))
    (:`2`
      ;[1 1 1] 2 Show Mate Picture
      (`/Game/UI/WBP_MainScreen.ShowMatePicture` (`self.Main UI`) true (`BlueprintMapLibrary.Map_Find` (`self.MatePictures`) (`self.SceneCounter`))))
    (:`3`
      ;[1 1 1] 3 Hide My Picture
      (`/Game/UI/WBP_MainScreen.ShowMyPicture` (`self.Main UI`) false))
    (:`4`
      ;[1 1 1] 4 Hide Mate Picture
      (`/Game/UI/WBP_MainScreen.ShowMatePicture` (`self.Main UI`) false null))
    (:`5`
      ;[1 1 1] 5 Set My Picture Editable
      (`/Game/UI/WBP_MainScreen.SetMyPicEditable` _main_ui true)
      (`/Game/UI/WBP_MainScreen.SetAvailableElements` _main_ui _output_elementset))
    (:`6`
      ;[1 1 1] 6 Set My Picture Disable Edit
      (`/Game/UI/WBP_MainScreen.SetMyPicEditable` (`self.Main UI`) false))
    (:`7`
      ;[1 1 1] 7 Clickable
      (`/Game/UI/WBP_MainScreen.ChangeClickableState` (`self.Main UI`) true))
    (:`8`
      ;[1 1 1] 8 Unclickable
      (`/Game/UI/WBP_MainScreen.ChangeClickableState` (`self.Main UI`) false))
    (:`9`
      ;[1 1 1] 9 MyPictureInit
      (`/Game/UI/WBP_MainScreen.MyPictureInit` (`self.Main UI`)))
    (:`10`
      ;[1 1 1] 10 INCREASE SCENE COUNTER
      (`/Engine/EditorBlueprintResources/StandardMacros.IncrementInt` (`self.SceneCounter`)))
    (:`12`
      ;[1 1 1] 12 To end
      (`GameplayStatics.OpenLevel` "Ending_P"))))