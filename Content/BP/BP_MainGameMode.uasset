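; Game mode that runs a branching, visual-novel style dialogue through the WBP_MainScreen widget it creates on BeginPlay.
; GoNextScene loads a data table row by jump index, splitting its backslash-delimited strings into lines, answers, next-row jumps and addon IDs for BPScenarioComponent.
; ShowNextLine advances the dialogue, showing answers with the last line and disabling click-through while a choice is pending.
; A Debug event sets the background and starts the first scene.
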(event `self.ReceiveBeginPlay`
  (bind _returnvalue (`|CreateWidget` "/Game/UI/WBP_MainScreen.WBP_MainScreen_C"))
  (bind _output_get (set `self.MainUI` _returnvalue))
  (`UserWidget.AddToViewport` _output_get 0)
  (`self.Debug`)
  (set `PlayerController.bShowMouseCursor` true (`GameplayStatics.GetPlayerController` 0))
  (`/Game/BP/BP_ScenarioComponent.Init` (`self.BP_ScenarioComponent`))
  ;[1 0.9242 0.2165] DEBUG
  (`/Game/UI/WBP_MainScreen.ShowMyPicture` (`self.MainUI`) false))

(event `GoNextScene`
  (params (RowNum :type Integer))
  (bind _output (`|GetArrayItem` (`self.NextSteps`) RowNum))
  (`/Game/UI/WBP_MainScreen.ChangeClickableState` (`self.MainUI`) true)
  (set `self.LinesCounter` 0)
  (bind _returnvalue (`|GetDataTableRow` "/Game/Data/NewDataTable.NewDataTable" (`KismetStringLibrary.Conv_StringToName` _output))
    (:`then`
      (bind (_charname _charlines _answers _charactersinscene _jumptostring _addon) (break `/Game/Data/Case_Str` _returnvalue))
      (`self.SetSpeakerName` _charname)
      (`self.SetCharLines` _charlines)
      (`self.SetAnswers` _answers)
      (set `self.Chars Array` _charactersinscene)
      (`self.SetJumps` _jumptostring)
      (set `self.CurrentRow` (`KismetStringLibrary.Conv_StringToInt` _output))
      (`self.ShowNextLine`)
      (`self.ActivateAddons` _addon))
    (:`RowNotFound`
      (`KismetSystemLibrary.PrintString` (`KismetTextLibrary.Conv_TextToString` (`|FormatText` "Oops, error in {RowNum}" (`self.CurrentRow`)))))))

(event `Debug`
  ;[1 0.8767 0.2531] Debug
  (`/Game/UI/WBP_MainScreen.SetBackground` (`self.MainUI`) (`self.BackgroundTexture`))
  (`self.GoNextScene` 0))

(event `ShowNextLine`
  (bind _mainui (`self.MainUI`))
  (bind _answers (`self.Answers`))
  (`/Game/UI/WBP_MainScreen.UpdateChars` (`self.MainUI`) (`self.Chars Array`))
  (bind _output_get (set `self.IsLastLine` (== (`KismetArrayLibrary.Array_LastIndex` (`self.DialogLines`)) (`self.LinesCounter`))))
  (if _output_get
    (`self.ClearDialog`)
    (`/Game/UI/WBP_MainScreen.ShowLastLineAndAnswers` _mainui (`|GetArrayItem` (`self.DialogLines`) (`self.LinesCounter`)) _answers)
    (if (not (`KismetArrayLibrary.Array_IsEmpty` _answers))
      ;[1 1 1] Wait For Player Choice
      (`/Game/UI/WBP_MainScreen.ChangeClickableState` _mainui false))
    (else
      (`/Game/UI/WBP_MainScreen.AddDialogLine` (`self.MainUI`) (`|GetArrayItem` (`self.DialogLines`) (`self.LinesCounter`)))
      (`/Engine/EditorBlueprintResources/StandardMacros.IncrementInt` (`self.LinesCounter`)))))

(event `ClearDialog`
  (`/Game/UI/WBP_MainScreen.ClearDialogWindow` (`self.MainUI`)))

(fn `ActivateAddons`
  (params (SourceString :type String))
  (bind _returnvalue (`KismetStringLibrary.ParseIntoArray` SourceString "\\"))
  (if (`KismetArrayLibrary.Array_IsNotEmpty` _returnvalue)
    (for _array_element _returnvalue
      (`/Game/BP/BP_ScenarioComponent.ActivateAddon` (`self.BP_ScenarioComponent`) (`KismetStringLibrary.Conv_StringToInt` _array_element)))))

(fn `SetAnswers`
  (params (SourceString :type String))
  (set `self.Answers` (`KismetStringLibrary.ParseIntoArray` SourceString "\\")))

(fn `SetCharLines`
  (params (SourceString :type String))
  (set `self.DialogLines` (`KismetStringLibrary.ParseIntoArray` SourceString "\\")))

(fn `SetJumps`
  (params (SourceString :type String))
  (set `self.NextSteps` (`KismetStringLibrary.ParseIntoArray` SourceString "\\")))

(fn `SetSpeakerName`
  (params (InString :type String))
  (`/Game/UI/WBP_MainScreen.SetSpeakerName` (`self.MainUI`) (`KismetTextLibrary.Conv_StringToText` InString)))

(fn `UserConstructionScript`)